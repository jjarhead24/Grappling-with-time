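; A door actor that starts or stays locked until its ButtonPressed flag, polled every tick, clears IsLocked.
; A box overlap toggles player input and shows either the first-person character's find-button or interact widget, depending on lock state.
; When unlocked, F plays a sound and a timeline that lerps the mesh upward.
; After five seconds a DoOnce guard resets and the timeline reverses to close it.
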(event `self.Box.OnComponentBeginOverlap`
  (params (OverlappedComponent :type "PrimitiveComponent Object Reference") (OtherActor :type "Actor Object Reference") (OtherComp :type "PrimitiveComponent Object Reference") (OtherBodyIndex :type Integer) (bFromSweep :type Boolean) (SweepResult :type "HitResult Structure (by ref)"))
  ;[1 1 1] when the player is in range let them press the button
  (bind _asfirst_person_character (cast `/Game/FirstPersonBP/Blueprints/FirstPersonCharacter` OtherActor))
  (`self.EnableInput` (`GameplayStatics.GetPlayerController` 0))
  (if (`self.IsLocked`)
    (bind _find_button (`/Game/FirstPersonBP/Blueprints/FirstPersonCharacter.find_button` _asfirst_person_character))
    ;[1 1 1] show find button message
    (if (not (`Widget.IsInViewport` _find_button))
      (`UserWidget.AddToViewport` _find_button 0))
    (else
      (bind _interact_message (`/Game/FirstPersonBP/Blueprints/FirstPersonCharacter.Interact_message` _asfirst_person_character))
      ;[1 1 1] show interact message
      (if (not (`Widget.IsInViewport` _interact_message))
        (`UserWidget.AddToViewport` _interact_message 0)))))

(event `self.Box.OnComponentEndOverlap`
  (params (OverlappedComponent :type "PrimitiveComponent Object Reference") (OtherActor :type "Actor Object Reference") (OtherComp :type "PrimitiveComponent Object Reference") (OtherBodyIndex :type Integer))
  ;[1 1 1] when the player is in range let them press the button
  (cast `/Game/FirstPersonBP/Blueprints/FirstPersonCharacter` OtherActor)
  (`self.DisableInput` (`GameplayStatics.GetPlayerController` 0))
  (if (`self.IsLocked`)
    (bind _find_button (`/Game/FirstPersonBP/Blueprints/FirstPersonCharacter.find_button` (stale `self.Box.OnComponentBeginOverlap` _asfirst_person_character)))
    ;[1 1 1] show find button message
    (if (`Widget.IsInViewport` _find_button)
      (`Widget.RemoveFromParent` _find_button))
    (else
      (bind _interact_message (`/Game/FirstPersonBP/Blueprints/FirstPersonCharacter.Interact_message` (stale `self.Box.OnComponentBeginOverlap` _asfirst_person_character)))
      ;[1 1 1] show interact message
      (if (`Widget.IsInViewport` _interact_message)
        (`Widget.RemoveFromParent` _interact_message)))))

(event `self.ReceiveTick`
  (params (DeltaSeconds :type "Float (single-precision)"))
  ;[1 1 1] every frame chack if the button has been pressed
  (if (`self.Button_pressed`)
    (set `self.IsLocked` false)))

(event `Key|F`
  (params (Key :type "Key Structure"))
  ;[1 1 1] Door Opener
  ;;[1 1 1] open the door, wait 5 seconds and close it
  (:`Pressed`
    (if (not (`self.IsLocked`))
      (`|ExecutionSequence`
        (:`then_0`
          (`/Engine/EditorBlueprintResources/StandardMacros.DoOnce` false :!label _label
            (:`Completed`
              (`GameplayStatics.PlaySoundAtLocation` "/Game/Audio/door_open.door_open" (`SceneComponent.K2_GetComponentLocation` (`self.Door`)) (struct) 1.0 1.0 0.0 null null null)
              ;;[1 1 1] timeline from 0 to 1 in a second
              (bind (_direction _open_close) (`Timeline|open/close` :!label _label_2)
                (:`Update`
                  ;;[1 1 1] move the door up into the roof
                  (`SceneComponent.K2_SetRelativeLocation` (`self.Cube`) (`KismetMathLibrary.VLerp` (0.0 0.0 0.0) (0.0 0.0 400.0) _open_close) false false))))))
        (:`then_1`
          (`KismetSystemLibrary.Delay` 5.0)
          (`|ExecutionSequence`
            (:`then_0`
              (goto _label :!via `Reset`))
            (:`then_1`
              (goto _label_2 :!via `Reverse`))))))))

(fn `GetStaticMeshComponent`
  (returns (StaticMesh :type "StaticMeshComponent Object Reference"))
  (return null))

(fn `Open_door1`)

(fn `UserConstructionScript`)
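; Wall-mounted button that lets the player trigger a door by pressing F while in range.
; A Box overlap with FirstPersonCharacter enables input and shows that character's InteractMessage widget, and leaving the box reverses both.
; Pressing F sets ButtonPressed to true on the referenced DoorOpening, with a DoOnce limiting the panel sound at the button's location to the first press.
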(event `Key|F`
  (params (Key :type "Key Structure"))
  ;[1 1 1] get user input
  (:`Pressed`
    ;[1 1 1] toggle the boolean so button pressed is true
    (set `/Game/Blueprints/BP_Door_button.Button_pressed` true (`self.Door_opening`))
    (`/Engine/EditorBlueprintResources/StandardMacros.DoOnce` false
      (:`Completed`
        (`GameplayStatics.PlaySoundAtLocation` "/Game/Audio/pannel_shot.pannel_shot" (`self.K2_GetActorLocation`) (struct) 1.0 1.0 0.5 null null null)))))

(event `self.Box.OnComponentBeginOverlap`
  (params (OverlappedComponent :type "PrimitiveComponent Object Reference") (OtherActor :type "Actor Object Reference") (OtherComp :type "PrimitiveComponent Object Reference") (OtherBodyIndex :type Integer) (bFromSweep :type Boolean) (SweepResult :type "HitResult Structure (by ref)"))
  ;[1 1 1] when the player is in range let them press the button
  (bind _asfirst_person_character (cast `/Game/FirstPersonBP/Blueprints/FirstPersonCharacter` OtherActor))
  (`self.EnableInput` (`GameplayStatics.GetPlayerController` 0))
  (bind _interact_message (`/Game/FirstPersonBP/Blueprints/FirstPersonCharacter.Interact_message` _asfirst_person_character))
  ;[1 1 1] show interact message
  (if (not (`Widget.IsInViewport` _interact_message))
    (`UserWidget.AddToViewport` _interact_message 0)))

(event `self.Box.OnComponentEndOverlap`
  (params (OverlappedComponent :type "PrimitiveComponent Object Reference") (OtherActor :type "Actor Object Reference") (OtherComp :type "PrimitiveComponent Object Reference") (OtherBodyIndex :type Integer))
  ;[1 1 1] when the player is in range let them press the button
  (cast `/Game/FirstPersonBP/Blueprints/FirstPersonCharacter` OtherActor)
  (`self.DisableInput` (`GameplayStatics.GetPlayerController` 0))
  (bind _interact_message (`/Game/FirstPersonBP/Blueprints/FirstPersonCharacter.Interact_message` (stale `self.Box.OnComponentBeginOverlap` _asfirst_person_character)))
  ;[1 1 1] show interact message
  (if (`Widget.IsInViewport` _interact_message)
    (`Widget.RemoveFromParent` _interact_message)))

(fn `UserConstructionScript`)
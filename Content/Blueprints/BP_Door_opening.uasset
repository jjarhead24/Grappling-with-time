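; Door Blueprint that slides open upward into the roof when the first-person character enters its trigger box.
; A timeline lerps the cube's relative height on begin overlap and reverses when the character leaves.
; A DoOnce limits the opening sound to one play until an end overlap resets it, which any actor can trigger because the reset precedes the character cast.
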(event `self.Box.OnComponentBeginOverlap`
  (params (OverlappedComponent :type "PrimitiveComponent Object Reference") (OtherActor :type "Actor Object Reference") (OtherComp :type "PrimitiveComponent Object Reference") (OtherBodyIndex :type Integer) (bFromSweep :type Boolean) (SweepResult :type "HitResult Structure (by ref)"))
  ;[1 1 1] check if the play is in range
  (cast `/Game/FirstPersonBP/Blueprints/FirstPersonCharacter` OtherActor)
  (`|ExecutionSequence`
    (:`then_0`
      (`/Engine/EditorBlueprintResources/StandardMacros.DoOnce` false :!label _label
        (:`Completed`
          (`GameplayStatics.PlaySoundAtLocation` "/Game/Audio/door_open.door_open" (`SceneComponent.K2_GetComponentLocation` (`self.Door`)) (struct) 1.0 1.0 0.0 null null null))))
    (:`then_1`
      ;[1 1 1] timeline from 0 to 1 in a second
      (bind (_direction _open_close) (`Timeline|open/close` :!label _label_2)
        (:`Update`
          ;[1 1 1] move the door up into the roof
          (`SceneComponent.K2_SetRelativeLocation` (`self.Cube`) (`KismetMathLibrary.VLerp` (0.0 0.0 0.0) (0.0 0.0 400.0) _open_close) false false))))))

(event `self.Box.OnComponentEndOverlap`
  (params (OverlappedComponent :type "PrimitiveComponent Object Reference") (OtherActor :type "Actor Object Reference") (OtherComp :type "PrimitiveComponent Object Reference") (OtherBodyIndex :type Integer))
  ;[1 1 1] check if the play is in range
  (`|ExecutionSequence`
    (:`then_0`
      (goto _label :!via `Reset`))
    (:`then_1`
      (cast `/Game/FirstPersonBP/Blueprints/FirstPersonCharacter` OtherActor)
      (goto _label_2 :!via `Reverse`))))

(fn `GetStaticMeshComponent`
  (returns (StaticMesh :type "StaticMeshComponent Object Reference"))
  (return null))

(fn `UserConstructionScript`)
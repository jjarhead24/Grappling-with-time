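; Screwy case actor that opens once, the first time the FirstPersonCharacter enters its Box trigger.
; The OpenCase timeline lerps the Glass and Er components upward along Z.
; On the first timeline update, a DoOnce plays the Gears sound at the actor and sets Opened.
; Box overlap also enables player input on the actor and disables it on exit, though the graph has no input events.
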(event `self.Box.OnComponentBeginOverlap`
  (params (OverlappedComponent :type "PrimitiveComponent Object Reference") (OtherActor :type "Actor Object Reference") (OtherComp :type "PrimitiveComponent Object Reference") (OtherBodyIndex :type Integer) (bFromSweep :type Boolean) (SweepResult :type "HitResult Structure (by ref)"))
  (cast `/Game/FirstPersonBP/Blueprints/FirstPersonCharacter` OtherActor)
  (`self.EnableInput` (`GameplayStatics.GetPlayerController` 0))
  (`/Engine/EditorBlueprintResources/StandardMacros.DoOnce` false
    (:`Completed`
      (bind (_direction _newtrack_0) (`Timeline|open case`)
        (:`Update`
          (`SceneComponent.K2_SetRelativeLocation` (`self.glass`) (`KismetMathLibrary.VLerp` (0.0 0.0 230.0) (0.0 0.0 400.0) _newtrack_0) false false)
          (`SceneComponent.K2_SetRelativeLocation` (`self.er`) (`KismetMathLibrary.VLerp` (0.0 0.0 1150.0) (0.0 0.0 1320.0) _newtrack_0) false false)
          (`/Engine/EditorBlueprintResources/StandardMacros.DoOnce` false
            (:`Completed`
              (`GameplayStatics.PlaySoundAtLocation` "/Game/Audio/gears.gears" (`self.K2_GetActorLocation`) (struct) 1.0 1.0 0.0 null null null)
              (set `self.opened` true))))))))

(event `Key|F`
  (params (Key :type "Key Structure")))

(event `self.Box.OnComponentEndOverlap`
  (params (OverlappedComponent :type "PrimitiveComponent Object Reference") (OtherActor :type "Actor Object Reference") (OtherComp :type "PrimitiveComponent Object Reference") (OtherBodyIndex :type Integer))
  (cast `/Game/FirstPersonBP/Blueprints/FirstPersonCharacter` OtherActor)
  (`self.DisableInput` (`GameplayStatics.GetPlayerController` 0)))

(fn `UserConstructionScript`)
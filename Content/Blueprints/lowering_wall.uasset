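; A wall actor that opens once the first-person character's PannelsShot count reaches NumPannelsNeeded, a threshold shown on its Number text.
; Tick polls the count and, while it is met, plays the open sound every frame and drives the DizzyOnTheComedown timeline.
; The timeline spins the cube and text and disables cube collision on its first update.
; When it finishes, an explosion spawns and the actor destroys itself.
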(event `self.ReceiveTick`
  (params (DeltaSeconds :type "Float (single-precision)"))
  (bind _asfirst_person_character (cast `/Game/FirstPersonBP/Blueprints/FirstPersonCharacter` (`GameplayStatics.GetPlayerCharacter` 0)))
  (if (>= (`/Game/FirstPersonBP/Blueprints/FirstPersonCharacter.pannels_shot` _asfirst_person_character) (`self.num_pannels_needed`))
    (`GameplayStatics.PlaySoundAtLocation` "/Game/Audio/wall_open.wall_open" (`self.K2_GetActorLocation`) (struct) 1.0 1.0 0.0 null null null)
    (bind (_direction _spin_with_me) (`Timeline|dizzy on the comedown`)
      (:`Update`
        (`SceneComponent.K2_SetRelativeRotation` (`self.Cube`) (`KismetMathLibrary.RLerp` (struct) (struct :`Pitch` 360.0 :`Yaw` 360.0 :`Roll` 360.0) _spin_with_me) false false)
        (`SceneComponent.K2_SetRelativeRotation` (`self.number`) (`KismetMathLibrary.RLerp` (struct) (struct :`Pitch` 360.0 :`Yaw` 360.0 :`Roll` 360.0) _spin_with_me) false false)
        (`/Engine/EditorBlueprintResources/StandardMacros.DoOnce` false
          (:`Completed`
            (`PrimitiveComponent.SetCollisionEnabled` (`self.Cube`) "NoCollision"))))
      (:`Finished`
        (`GameplayStatics.SpawnEmitterAtLocation` "/Game/StarterContent/Particles/P_Explosion.P_Explosion" (`SceneComponent.K2_GetComponentLocation` (`self.Cube`)))
        (`self.K2_DestroyActor`)))))

(event `self.ReceiveBeginPlay`
  (`TextRenderComponent.K2_SetText` (`self.number`) (`KismetTextLibrary.Conv_IntToText` (`self.num_pannels_needed`))))

(fn `UserConstructionScript`)
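; Enemy turret that turns to face the first-person player it sees via PawnSensing and fires projectiles from Firepoint on a one-second cooldown.
; Player projectile overlaps on the capsule apply damage to itself; AnyDamage explodes and destroys it if Damage minus CurrentHealth is zero or less, without updating health.
; A Box overlap starts a 2D engine sound through a DoOnce that resets after a delay, and leaving stops it.
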(event `self.PawnSensing.OnSeePawn`
  (params (Pawn :type "Pawn Object Reference"))
  ;[1 1 1] turret looks at the player
  (bind _asfirst_person_character (cast `/Game/FirstPersonBP/Blueprints/FirstPersonCharacter` Pawn))
  (`|ExecutionSequence`
    (:`then_0`
      (`self.K2_SetActorRotation` (`KismetMathLibrary.FindLookAtRotation` (`self.K2_GetActorLocation`) (`self.K2_GetActorLocation` _asfirst_person_character))))
    (:`then_1`
      ;[1 1 1] fire projectile
      (if (`self.spawn projectile`)
        (`|SpawnActorFromClass` "/Game/FirstPersonBP/Blueprints/enemy_proj.enemy_proj_C" (`SceneComponent.K2_GetComponentToWorld` (`self.firepoint`)) "Undefined" "OverrideRootScale" null null)
        (`GameplayStatics.PlaySoundAtLocation` "/Game/FirstPersonBP/Blueprints/boing.boing" (`self.K2_GetActorLocation`) (struct) 1.0 1.0 0.0 null null null)
        (set `self.spawn projectile` false)
        (`KismetSystemLibrary.Delay` 1.0)
        (set `self.spawn projectile` true)))))

(event `self.ReceiveAnyDamage`
  (params (Damage :type "Float (single-precision)") (DamageType :type "DamageType Object Reference") (InstigatedBy :type "Controller Object Reference") (DamageCauser :type "Actor Object Reference"))
  (bind _returnvalue (`SceneComponent.K2_GetComponentLocation` (`self.CapsuleComponent`)))
  ;[1 1 1] damage handler
  (if (<= (- Damage (`self.current health`)) 0.0)
    (`GameplayStatics.SpawnEmitterAtLocation` "/Game/StarterContent/Particles/P_Explosion.P_Explosion" _returnvalue)
    (`GameplayStatics.SpawnEmitterAtLocation` "/Game/MaterialFunctionCollection/ShowcaseAssets/ExampleContent/Effects/P_Pulse_Ring.P_Pulse_Ring" _returnvalue)
    (`GameplayStatics.SpawnEmitterAtLocation` "/Game/Polar/Particles/P_Clouds.P_Clouds" _returnvalue)
    (`GameplayStatics.SpawnEmitterAtLocation` "/Game/Polar/Particles/P_Sparks_Dense.P_Sparks_Dense" _returnvalue)
    (`GameplayStatics.PlaySoundAtLocation` "/Game/Audio/explosion.explosion" (`self.K2_GetActorLocation`) (struct) 1.0 1.0 0.0 null null null)
    (`self.K2_DestroyActor`)))

(event `self.CapsuleComponent.OnComponentBeginOverlap`
  (params (OverlappedComponent :type "PrimitiveComponent Object Reference") (OtherActor :type "Actor Object Reference") (OtherComp :type "PrimitiveComponent Object Reference") (OtherBodyIndex :type Integer) (bFromSweep :type Boolean) (SweepResult :type "HitResult Structure (by ref)"))
  ;[1 1 1] apply damage#
  (cast `/Game/FirstPersonBP/Blueprints/FirstPersonProjectile` OtherActor)
  (`GameplayStatics.ApplyDamage` self 100.0))

(event `self.Box.OnComponentBeginOverlap`
  (params (OverlappedComponent :type "PrimitiveComponent Object Reference") (OtherActor :type "Actor Object Reference") (OtherComp :type "PrimitiveComponent Object Reference") (OtherBodyIndex :type Integer) (bFromSweep :type Boolean) (SweepResult :type "HitResult Structure (by ref)"))
  ;[1 1 1] engine sound
  (cast `/Game/FirstPersonBP/Blueprints/FirstPersonCharacter` OtherActor)
  (`/Engine/EditorBlueprintResources/StandardMacros.DoOnce` false :!label _label
    (:`Completed`
      (bind _returnvalue (`GameplayStatics.SpawnSound2D` "/Game/Audio/turret_engine.turret_engine" 0.05 1.0 0.0 null false false))
      (bind _output_get (set `self.sound` _returnvalue))
      (`AudioComponent.Play` _output_get 0.0)
      (`KismetSystemLibrary.Delay` 16.9)
      (set `self.play sound?` true)
      (if (`self.play sound?`)
        (goto _label :!via `Reset`)))))

(event `self.Box.OnComponentEndOverlap`
  (params (OverlappedComponent :type "PrimitiveComponent Object Reference") (OtherActor :type "Actor Object Reference") (OtherComp :type "PrimitiveComponent Object Reference") (OtherBodyIndex :type Integer))
  (cast `/Game/FirstPersonBP/Blueprints/FirstPersonCharacter` OtherActor)
  (set `self.play sound?` false)
  (`AudioComponent.Stop` (`self.sound`))
  (goto _label :!via `Reset`))

(fn `UserConstructionScript`)
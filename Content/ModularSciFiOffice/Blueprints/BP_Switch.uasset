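; Interactable switch actor that triggers linked usable actors and can teleport the player or load another level.
; Focus toggles a custom-depth stencil highlight on the switch mesh.
; Use sends UseMessage to UsableActors through the BP_UsableActor interface, optionally flipping the emissive tint between green and red via a dynamic material.
; After a delay, it teleports the player or opens the named level, but only when UsableActors is non-empty.
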(event `self.ReceiveBeginPlay`
  (bind _switch (`self.Switch`))
  (bind _returnvalue (`PrimitiveComponent.CreateDynamicMaterialInstance` _switch 0 (`PrimitiveComponent.GetMaterial` _switch 0)))
  (set `self.MaterialInstance` _returnvalue)
  (if (`self.ChangeColor`)
    (`MaterialInstanceDynamic.SetVectorParameterValue` (`self.MaterialInstance`) "EmissiveTint" (struct :`G` 1.0 :`A` 1.0))))

(event `/Game/ModularSciFiOffice/Blueprints/BP_UsableActor.StartFocus`
  (`PrimitiveComponent.SetCustomDepthStencilValue` (`self.Switch`) 252)
  (`PrimitiveComponent.SetRenderCustomDepth` (`self.Switch`) true))

(event `/Game/ModularSciFiOffice/Blueprints/BP_UsableActor.StopFocus`
  (`PrimitiveComponent.SetRenderCustomDepth` (`self.Switch`) false))

(event `/Game/ModularSciFiOffice/Blueprints/BP_UsableActor.Use`
  (params (IsPlayer :type Boolean))
  (bind _isopened (`self.IsOpened`))
  (bind _usableactors (`self.UsableActors`))
  (bind _returnvalue (not _isopened))
  (bind _returnvalue_2 (`KismetStringLibrary.Trim` (`KismetStringLibrary.Conv_NameToString` (`self.Level`))))
  (if (> (`KismetArrayLibrary.Array_Length` _usableactors) 0)
    (for _array_element _usableactors
      (`/Engine/EditorBlueprintResources/StandardMacros.IsValid` _array_element
        (:`Is Valid`
          (if (`KismetSystemLibrary.DoesImplementInterface` _array_element "/Game/ModularSciFiOffice/Blueprints/BP_UsableActor.BP_UsableActor_C")
            (message `/Game/ModularSciFiOffice/Blueprints/BP_UsableActor.Use` _array_element false)))))
    (if (`self.ChangeColor`)
      (if _isopened
        (set `self.IsOpened` _returnvalue)
        (`MaterialInstanceDynamic.SetVectorParameterValue` (`self.MaterialInstance`) "EmissiveTint" (struct :`R` 1.0 :`A` 1.0))
        (else
          (set `self.IsOpened` _returnvalue)
          (`MaterialInstanceDynamic.SetVectorParameterValue` (`self.MaterialInstance`) "EmissiveTint" (struct :`G` 1.0 :`A` 1.0)))))
    (`KismetSystemLibrary.Delay` (`self.TranslationDelay`))
    (if (`self.Teleport`)
      (`self.K2_SetActorLocation` (`GameplayStatics.GetPlayerPawn` 0) (`self.TeleportLocation`) false true)
      (`self.K2_SetActorRotation` (`GameplayStatics.GetPlayerPawn` 0) (`self.TeleportRotation`) true)
      (`Controller.SetControlRotation` (`GameplayStatics.GetPlayerController` 0) (`self.TeleportRotation`))
      (elif (`self.ChangeLevel`)
        (if (and (`KismetStringLibrary.NotEqual_StrStr` _returnvalue_2) (`KismetStringLibrary.NotEqual_StrStr` _returnvalue_2))
          (`GameplayStatics.OpenLevel` (`self.Level`)))))))

(fn `GetStaticMeshComponent`
  (returns (StaticMesh :type "StaticMeshComponent Object Reference"))
  (return null))

(fn `UserConstructionScript`)